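; Snow Niagara actor that follows the player pawn at an offset each Tick, adapting snowfall and fog to how sheltered the player is.
; CeilingCheck traces a grid of rays from the actor's position and returns, and debug-prints, the fraction that hit.
; The inverse drives the Niagara SnowAlpha and, scaled by trigger-set BlizzardStrength, a squared lerp for exponential height fog density.
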(event EventBeginPlay)

(event EventTick
  (params (DeltaSeconds :type Float%20%28single-precision%29))
  (bind _returnvalue (Game|Player|GetPlayerPawn 0))
  (bind _playeroffset (Variables|Default|GetPlayerOffset))
  (bind _returnvalue_2 (Transformation|GetActorLocation _returnvalue))
  (bind _returnvalue_3 (+ _returnvalue_2 _playeroffset))
  ;[0.15 0.03713 0.07684] Move Emitter Abobe Player
  (Transformation|SetActorLocation _returnvalue_3 false false)
  (bind _indoorspercentage (CallFunction|CeilingCheck _returnvalue_3 7 7))
  (Niagara|SetNiagaraVariable(Float) (Variables|NiagaraActor|GetNiagaraComponent) "SnowAlpha" (- 1.0 _indoorspercentage))
  (Class|ExponentialHeightFogComponent|SetFogDensity (Variables|Default|GetExponentialHeightFog) (* (Math|Float|Lerp 0.05 0.8 (* (- 1.0 _indoorspercentage) (Variables|Default|GetblizzardStrength))) (Math|Float|Lerp 0.05 0.8 (* (- 1.0 _indoorspercentage) (Variables|Default|GetblizzardStrength))))))

(fn ConstructionScript)

(fn CeilingCheck
  (params (PlayerPos :type Vector) (AmountX :type Integer) (AmountY :type Integer))
  (bind _returnvalue (+ AmountX 1))
  (bind _returnvalue_2 (+ AmountY 1))
  (bind _rayshit (LocalVariables|GetRaysHit))
  (bind _returnvalue_3 (Math|Conversions|ToFloat(Integer) _rayshit))
  (bind _returnvalue_4 (* _returnvalue _returnvalue_2))
  (bind _returnvalue_5 (Math|Conversions|ToFloat(Integer) _returnvalue_4))
  (bind _returnvalue_6 (/ _returnvalue_3 _returnvalue_5))
  ;[0.15 0.15 0.15 0.5] Create a grid offset
  (for _index (range 0 AmountX)
    (for _index_2 (range 0 AmountY)
      ;[0.15 0.133 0.07744 0.5] Raycast for each in grid
      (bind _returnvalue_7 (Class|KismetSystemLibrary|LineTraceSinglebyProfile (+ PlayerPos (Math|Vector|MakeVector (* (Variables|Default|GetIndoorsCheckRaySpread) (|(A-(B/2)) (Math|Conversions|ToFloat(Integer) _index) (Math|Conversions|ToFloat(Integer) AmountX))) (* (|(A-(B/2)) (Math|Conversions|ToFloat(Integer) _index_2) (Math|Conversions|ToFloat(Integer) AmountY)) (Variables|Default|GetIndoorsCheckRaySpread)) 0.0)) (+ PlayerPos (Math|Vector|MakeVector (* (Variables|Default|GetIndoorsCheckRaySpread) (|(A-(B/2)) (Math|Conversions|ToFloat(Integer) _index) (Math|Conversions|ToFloat(Integer) AmountX))) (* (|(A-(B/2)) (Math|Conversions|ToFloat(Integer) _index_2) (Math|Conversions|ToFloat(Integer) AmountY)) (Variables|Default|GetIndoorsCheckRaySpread)) 0.0) (Variables|Default|GetIndoorsCheckRayDirection)) "None" false (Utilities|Array|MakeArray (Game|Player|GetPlayerPawn 0)) "None" true))
      (if _returnvalue_7
        (bind _result (Math|Integer|IncrementInt (LocalVariables|GetRaysHit))))))
  (Development|PrintString (Class|KismetStringLibrary|BuildStringDouble (LocalVariables|GetOutdoorString) "" _returnvalue_6) true true "(R=0.208343,G=0.334235,B=1.000000,A=1.000000)" 0.0)
  (return _returnvalue_6))